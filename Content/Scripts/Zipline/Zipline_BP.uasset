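; Zipline actor that strings a cable between a start and end post and offers the ride to overlapping actors.
; InitCable, run at construction and BeginPlay, moves the cable to the start top and attaches its end to the end top.
; Each end's collision sends SetZiplineMessage with travel start and end positions, clearing it on exit.
; The start end always enables travel; the far end only when BothWays is set.
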(event OnComponentBeginOverlap(Start_Collision)
  (params (OverlappedComponent :type Primitive%20Component%20Object%20Reference) (OtherActor :type Actor%20Object%20Reference) (OtherComp :type Primitive%20Component%20Object%20Reference) (OtherBodyIndex :type Integer) (bFromSweep :type Boolean) (SweepResult :type Hit%20Result%20Structure%20%28by%20ref%29))
  (Class|ZiplineBPI|SetZipline(Message) OtherActor true (Transformation|GetWorldLocation (Variables|Default|GetStart_Collision)) (Transformation|GetWorldLocation (Variables|Default|GetEnd_Collision))))

(event OnComponentEndOverlap(Start_Collision)
  (params (OverlappedComponent :type Primitive%20Component%20Object%20Reference) (OtherActor :type Actor%20Object%20Reference) (OtherComp :type Primitive%20Component%20Object%20Reference) (OtherBodyIndex :type Integer))
  (Class|ZiplineBPI|SetZipline(Message) OtherActor false "0, 0, 0" "0, 0, 0"))

(event OnComponentBeginOverlap(End_Collision)
  (params (OverlappedComponent :type Primitive%20Component%20Object%20Reference) (OtherActor :type Actor%20Object%20Reference) (OtherComp :type Primitive%20Component%20Object%20Reference) (OtherBodyIndex :type Integer) (bFromSweep :type Boolean) (SweepResult :type Hit%20Result%20Structure%20%28by%20ref%29))
  (Class|ZiplineBPI|SetZipline(Message) OtherActor (Variables|Default|GetBoth%20Ways?) (Transformation|GetWorldLocation (Variables|Default|GetEnd_Collision)) (Transformation|GetWorldLocation (Variables|Default|GetStart_Collision))))

(event OnComponentEndOverlap(End_Collision)
  (params (OverlappedComponent :type Primitive%20Component%20Object%20Reference) (OtherActor :type Actor%20Object%20Reference) (OtherComp :type Primitive%20Component%20Object%20Reference) (OtherBodyIndex :type Integer))
  (Class|ZiplineBPI|SetZipline(Message) OtherActor false "0, 0, 0" "0, 0, 0"))

(event EventBeginPlay
  (Utilities|InitCable))

(event Collision|EventActorBeginOverlap
  (params (OtherActor :type Actor%20Object%20Reference)))

(event EventTick
  (params (DeltaSeconds :type Float%20%28single-precision%29)))

(fn ConstructionScript
  (Utilities|InitCable))