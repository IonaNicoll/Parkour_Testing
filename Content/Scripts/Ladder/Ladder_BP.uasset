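; Procedural ladder actor that sizes itself from a Height value and tells overlapping actors when they can use it.
; InitLadder, run in the Construction Script and at BeginPlay, moves LadderTop, then centers and stretches both side rails and the collider to match.
; Crossbars are rebuilt as instanced static meshes spaced by CrossbarGap.
; The collider sends SetLadderMessage to the other actor, passing itself on begin overlap and nothing on end.
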(event OnComponentBeginOverlap(LadderCollider)
  (params (OverlappedComponent :type Primitive%20Component%20Object%20Reference) (OtherActor :type Actor%20Object%20Reference) (OtherComp :type Primitive%20Component%20Object%20Reference) (OtherBodyIndex :type Integer) (bFromSweep :type Boolean) (SweepResult :type Hit%20Result%20Structure%20%28by%20ref%29))
  (Class|ClimbingBPI|SetLadder(Message) OtherActor self))

(event OnComponentEndOverlap(LadderCollider)
  (params (OverlappedComponent :type Primitive%20Component%20Object%20Reference) (OtherActor :type Actor%20Object%20Reference) (OtherComp :type Primitive%20Component%20Object%20Reference) (OtherBodyIndex :type Integer))
  (Class|ClimbingBPI|SetLadder(Message) OtherActor))

(event Custom|Init%20Ladder
  (bind _ism_crossbar (Variables|Default|Getism_Crossbar))
  (Transformation|SetRelativeLocation (Variables|Default|GetLadder%20Top) (Math|Vector|MakeVector 0.0 0.0 (Variables|Default|GetHeight)) false false)
  (Utilities|AdjustRightBar (Variables|Default|GetLadder_R))
  (Utilities|AdjustLeftBar (Variables|Default|GetLadder_L))
  (Utilities|AdjustLeftBar (Variables|Default|GetLadder%20Collider))
  (Variables|Default|SetTemp_Height 0.0)
  (Components|InstancedStaticMesh|ClearInstances _ism_crossbar)
  (while (< (Variables|Default|GetTemp_Height) (.z (Variables|/Script/Engine.SceneComponent|GetRelativeLocation (Variables|Default|GetLadder%20Top))))
    (Components|InstancedStaticMesh|AddInstance _ism_crossbar (Math|Transform|MakeTransform (Math|Vector|MakeVector 0.0 0.0 (Variables|Default|GetTemp_Height)) "0, 0, 0" "0.050000,0.600000,0.050000"))
    (Variables|Default|SetTemp_Height (+ (Variables|Default|GetTemp_Height) (Variables|Default|GetCrossbar%20Gap)))))

(event EventBeginPlay
  (CallFunction|InitLadder))

(event Collision|EventActorBeginOverlap
  (params (OtherActor :type Actor%20Object%20Reference)))

(event EventTick
  (params (DeltaSeconds :type Float%20%28single-precision%29)))

(fn ConstructionScript
  (CallFunction|InitLadder))